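; Player 1's Paper2D side-scrolling character, with axis movement, jumping by key or touch, and a points counter.
; Tick flips facing by X velocity and sets the flipbook from the States variable.
; Landing resets the state, with a short delay before restoring input after a hit.
; An airborne upward damage trace (Dano) leaves its result unused; crouch logic is disconnected and Sprint is empty.
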(event Custom|UpdateAnimation
  ;[1 1 1] Handle Animation
  (switch Utilities|FlowControl|Switch|Switchonstates_player (Variables|Default|Getstates)
    (:NewEnumerator0
      (Sprite|SetFlipbook (Variables|Default|GetSprite) (select (> (Math|Vector|VectorLength (Transformation|GetVelocity)) 0.0) "/Game/JumpOver/Sprites2/Frames/Player1/p1_walk_v2.p1_walk_v2" "/Game/JumpOver/Sprites2/Frames/Player1/p1_idle_v2.p1_idle_v2")))
    (:NewEnumerator1
      (Sprite|SetFlipbook (Variables|Default|GetSprite) "/Game/JumpOver/Sprites2/Frames/Player1/p1_jump_v2.p1_jump_v2"))
    (:NewEnumerator4
      (Sprite|SetFlipbook (Variables|Default|GetSprite) "/Game/JumpOver/Sprites2/Frames/Player1/p1_hit_v2.p1_hit_v2"))))

(event Custom|Event%20Dano
  (bind _self self)
  (bind _returnvalue (Transformation|GetActorLocation _self))
  ;[1 1 1] Event Dano
  (if (not (AI|Components|NavMovement|IsMovingonGround (Variables|Character|GetCharacterMovement)))
    (bind _outhit (Collision|LineTraceForObjects _returnvalue (+ _returnvalue (* (Transformation|GetActorUpVector _self) (Variables|Default|GetTraceLength))) (Utilities|Array|MakeArray "ObjectTypeQuery1" "ObjectTypeQuery3") false 0 "None"))))

(event Custom|Points%20System
  (params (Valor :type Integer))
  ;[1 1 1] Points System
  (Variables|Default|Setpontos (+ Valor (Variables|Default|Getpontos))))

(event EventTick
  (params (DeltaSeconds :type Float%20%28single-precision%29))
  ;[1 1 1] Tick - Updates animation
  (Utilities|FlowControl|Sequence
    (:then_0
      (CallFunction|EventDano))
    (:then_1
      (CallFunction|UpdateAnimation)
      (Math|Float|CompareFloat (.X (Math|Vector|BreakVector (Variables|/Script/Engine.MovementComponent|GetVelocity (Pawn|GetMovementComponent)))) 0.0
        (:>
          (Pawn|SetControlRotation (Pawn|GetController) (Math|Rotator|MakeRotator 0.0 0.0 0.0))
          (Variables|Default|Setfacing 1))
        (:<
          (Pawn|SetControlRotation (Pawn|GetController) (Math|Rotator|MakeRotator 0.0 0.0 1.8e+02))
          (Variables|Default|Setfacing -1))))))

(event EventOnLanded
  (params (Hit :type Hit%20Result%20Structure%20%28by%20ref%29))
  ;[1 1 1] Evento ao Aterrissar
  (if (Variables|Default|GetisHit)
    (Variables|Default|Setstates "NewEnumerator5")
    (CallFunction|UpdateAnimation)
    (Utilities|FlowControl|Delay 0.5)
    (Variables|Default|Setstates "NewEnumerator0")
    (CallFunction|UpdateAnimation)
    (Input|EnableInput (Game|GetPlayerController 0))
    (Variables|Default|SetisHit false)
    (else
      (Variables|Default|Setstates "NewEnumerator0")
      (CallFunction|UpdateAnimation))))

(event EventBeginPlay
  (Class|ActorComponent|SetIsReplicated (Variables|Default|GetSprite) true))

(event Input|ActionEvents|InputActionAgachar
  (params (Key :type Key%20Structure :default "AnyKey"))
  ;[1 1 1] Agachar
)

(event Input|ActionEvents|InputActionJump
  (params (Key :type Key%20Structure :default "AnyKey"))
  ;[1 1 1] Handle Jump
  (:Pressed
    (Character|Jump)
    (Variables|Default|Setstates "NewEnumerator1"))
  (:Released
    (Character|StopJumping)))

(event Input|AxisEvents|InputAxisMoveRight
  (params (AxisValue :type Float%20%28single-precision%29))
  (bind _velocidade (Variables|Default|Getvelocidade))
  ;[1 1 1] Handle movement
  (Pawn|Input|AddMovementInput "1.000000, 0, 0" (* (/ AxisValue (Variables|Default|Getvelocidade)) (Math|Float|Clamp(Float) (* (stale Input|AxisEvents|InputAxisSprint AxisValue) _velocidade) (Variables|Default|GetvelocidadeCaminhando) _velocidade)) false))

(event Input|AxisEvents|InputAxisSprint
  (params (AxisValue :type Float%20%28single-precision%29))
  ;[1 1 1] Handle movement
)

(event Input|TouchEvents|InputTouch
  (params (Location :type Vector) (FingerIndex :type ETouchIndex%20Enum))
  ;[1 1 1] Handle Jump
  (:Pressed
    (Character|Jump)
    (Variables|Default|Setstates "NewEnumerator1"))
  (:Released
    (Character|StopJumping)))

(fn ConstructionScript)