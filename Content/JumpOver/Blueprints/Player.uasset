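; Player Paper2D character for the JumpOver side-scroller, with axis movement, key or touch jumping, and state-driven flipbook animation.
; BeginPlay stores the spawn transform in the game mode, switches view to the active world camera and creates the HUD.
; While airborne, a vertical line trace kills hit manual-AI enemies, matched by class name, and adds a point.
; Death launches the player with collision off, then hides it and calls CallKillPlayer; crouch logic is unconnected.
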(event Custom|UpdateAnimation
  ;[1 1 1] Handle Animation
  (switch Utilities|FlowControl|Switch|Switchonstates_player (Variables|Default|Getstates)
    (:NewEnumerator0
      (Sprite|SetFlipbook (Variables|Default|GetSprite) (select (> (Math|Vector|VectorLength (Transformation|GetVelocity)) 0.0) "/Game/JumpOver/Sprites2/Frames/p1_walk_v2.p1_walk_v2" "/Game/JumpOver/Sprites2/Frames/p1_idle_v2.p1_idle_v2")))
    (:NewEnumerator1
      (Sprite|SetFlipbook (Variables|Default|GetSprite) "/Game/JumpOver/Sprites2/Frames/p1_jump_v2.p1_jump_v2"))
    (:NewEnumerator4
      (Sprite|SetFlipbook (Variables|Default|GetSprite) "/Game/JumpOver/Sprites2/Frames/p1_hit_v2.p1_hit_v2"))))

(event Custom|Event%20Dano
  (bind _self self)
  (bind _returnvalue (Transformation|GetActorLocation _self))
  ;[1 1 1] Event Dano
  (if (not (AI|Components|NavMovement|IsMovingonGround (Variables|Character|GetCharacterMovement)))
    (if (Variables|Default|GethitEnable)
      (bind _outhit (Collision|LineTraceForObjects _returnvalue (+ _returnvalue (* (Transformation|GetActorUpVector _self) (Variables|Default|GetTraceLength))) (Utilities|Array|MakeArray "ObjectTypeQuery1" "ObjectTypeQuery3") false 0 "ForOneFrame"))
      (if (Math|Boolean|Equal(Boolean) (Utilities|ClassIsChildOf (Utilities|GetClass (.HitActor (Collision|BreakHitResult _outhit))) "/Script/Paper2D.PaperCharacter") true)
        (Development|PrintString (Utilities|GetClassDisplayName (Utilities|GetClass (.HitActor (Collision|BreakHitResult _outhit)))))
        (switch string (Utilities|GetClassDisplayName (Utilities|GetClass (.HitActor (Collision|BreakHitResult _outhit))))
          (:EnemyAIManual_C
            (bind _asenemy_aimanual (Utilities|Casting|CastToEnemyAIManual (.HitActor (Collision|BreakHitResult _outhit))))
            (Default|KillBotEvent _asenemy_aimanual)
            (Math|Integer|IncrementInt (Variables|Default|Getpontos))))))))

(event Custom|Kill%20Player_Event
  (Variables|Default|SethitEnable false)
  (Physics|AddImpulse (Variables|Character|GetCharacterMovement) (Math|Vector|MakeVector (* (Variables|Default|Getfacing) 1e+04) 0.0 2e+04) false)
  (Collision|SetActorEnableCollision false)
  (Variables|Default|Setstates "NewEnumerator4")
  (CallFunction|UpdateAnimation)
  (Utilities|FlowControl|Delay 1.0)
  (Rendering|SetActorHiddenInGame true)
  (Game|Player|SetViewTargetwithBlend (Game|GetPlayerController 0) (Variables|Default|GetWorldCamera) 0.0 "VTBlend_Linear" 0.0 false)
  (Default|CallKillPlayer))

(event Custom|Points%20System
  (params (Valor :type Integer))
  ;[1 1 1] Points System
  (Variables|Default|Setpontos (+ Valor (Variables|Default|Getpontos))))

(event Custom|Find%20World%20Camera
  (bind _outactors (Actor|GetAllActorsOfClass "/Game/JumpOver/Blueprints/CameraBP.CameraBP_C"))
  (for _array_element _outactors
    (if (Components|Activation|IsActive (Variables|/Script/Engine.CameraActor|GetCameraComponent _array_element))
      (bind _output_get (Variables|Default|SetWorldCamera _array_element))
      (Game|Player|SetViewTargetwithBlend (Game|GetPlayerController 0) _output_get 0.0 "VTBlend_Linear" 0.0 false))))

(event EventTick
  (params (DeltaSeconds :type Float%20%28single-precision%29))
  ;[1 1 1] Tick - Updates animation
  (Utilities|FlowControl|Sequence
    (:then_0
      (CallFunction|EventDano))
    (:then_1
      (CallFunction|UpdateAnimation)
      (Math|Float|CompareFloat (.X (Math|Vector|BreakVector (Variables|/Script/Engine.MovementComponent|GetVelocity (Pawn|GetMovementComponent)))) 0.0
        (:>
          (Pawn|SetControlRotation (Pawn|GetController) (Math|Rotator|MakeRotator 0.0 0.0 0.0))
          (Variables|Default|Setfacing 1))
        (:<
          (Pawn|SetControlRotation (Pawn|GetController) (Math|Rotator|MakeRotator 0.0 0.0 1.8e+02))
          (Variables|Default|Setfacing -1))))))

(event EventOnLanded
  (params (Hit :type Hit%20Result%20Structure%20%28by%20ref%29))
  ;[1 1 1] Evento ao Aterrissar
  (if (Variables|Default|GetisHit)
    (Variables|Default|Setstates "NewEnumerator5")
    (CallFunction|UpdateAnimation)
    (Utilities|FlowControl|Delay 0.5)
    (Variables|Default|Setstates "NewEnumerator0")
    (CallFunction|UpdateAnimation)
    (Input|EnableInput (Game|GetPlayerController 0))
    (Variables|Default|SetisHit false)
    (else
      (Variables|Default|Setstates "NewEnumerator0")
      (CallFunction|UpdateAnimation))))

(event EventBeginPlay
  (Utilities|FlowControl|Sequence
    (:then_0
      (Class|ActorComponent|SetIsReplicated (Variables|Default|GetSprite) true))
    (:then_1
      (bind _asgame_mode_jump_over (Utilities|Casting|CastToGameModeJumpOver (Game|GetGameMode)))
      (Variables|/Game/JumpOver/Blueprints/GameModeJumpOver.GameModeJumpOver_C|SetSpawn%20Transform _asgame_mode_jump_over (Transformation|GetActorTransform)))
    (:then_2
      (CallFunction|FindWorldCamera))
    (:then_3
      (bind _returnvalue (UserInterface|CreateWidget "/Game/JumpOver/Blueprints/HUD/MainHUD.MainHUD_C" (Game|GetPlayerController 0)))
      (bind _output_get (Variables|Default|SetHUDPlayer _returnvalue))
      (UserInterface|Viewport|AddtoViewport _output_get 0))))

(event Input|ActionEvents|InputActionAgachar
  (params (Key :type Key%20Structure :default "AnyKey"))
  ;[1 1 1] Agachar
)

(event Input|ActionEvents|InputActionJump
  (params (Key :type Key%20Structure :default "AnyKey"))
  ;[1 1 1] Handle Jump
  (:Pressed
    (Character|Jump)
    (Variables|Default|Setstates "NewEnumerator1"))
  (:Released
    (Character|StopJumping)))

(event Input|AxisEvents|InputAxisMoveRight
  (params (AxisValue :type Float%20%28single-precision%29))
  (bind _velocidade (Variables|Default|Getvelocidade))
  ;[1 1 1] Handle movement
  (Pawn|Input|AddMovementInput "1.000000, 0, 0" (* (/ AxisValue (Variables|Default|Getvelocidade)) (Math|Float|Clamp(Float) (* (stale Input|AxisEvents|InputAxisSprint AxisValue) _velocidade) (Variables|Default|GetvelocidadeCaminhando) _velocidade)) false))

(event Input|AxisEvents|InputAxisSprint
  (params (AxisValue :type Float%20%28single-precision%29))
  ;[1 1 1] Handle movement
)

(event Input|TouchEvents|InputTouch
  (params (Location :type Vector) (FingerIndex :type ETouchIndex%20Enum))
  ;[1 1 1] Handle Jump
  (:Pressed
    (Character|Jump)
    (Variables|Default|Setstates "NewEnumerator1"))
  (:Released
    (Character|StopJumping)))

(fn ConstructionScript)