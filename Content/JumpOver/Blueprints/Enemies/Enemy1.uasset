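; Enemy1 is a Paper2D character Blueprint for a jumping enemy, with flipbook animation driven by a States variable.
; Tick refreshes the animation, turns the controller to face horizontal velocity and, while airborne, traces upward, only printing the hit actor's name.
; Landing resets the state, adding a short Standing recovery and re-enabling player input after a hit.
; A points adder exists, and the jump logic is unconnected.
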(event Custom|Dano%20Event
  (bind _self self)
  (bind _returnvalue (Transformation|GetActorLocation _self))
  ;[1 1 1] Dano Event
  (if (not (AI|Components|NavMovement|IsMovingonGround (Variables|Character|GetCharacterMovement)))
    (bind _outhit (Collision|LineTraceForObjects _returnvalue (+ _returnvalue (* (Transformation|GetActorUpVector _self) (Variables|Default|GetTraceLength))) (Utilities|Array|MakeArray "ObjectTypeQuery1" "ObjectTypeQuery3") false 0 "None"))
    (Development|PrintString (Utilities|GetDisplayName (.HitActor (Collision|BreakHitResult _outhit))))))

(event Custom|UpdateAnimation
  ;[1 1 1] Handle Animation
  (switch Utilities|FlowControl|Switch|Switchonstates_player (Variables|Default|Getstates)
    (:NewEnumerator0
      (Sprite|SetFlipbook (Variables|Default|GetSprite) (select (> (Math|Vector|VectorLength (Transformation|GetVelocity)) 0.0) "/Game/JumpOver/Sprites/Players/Player2/p2_walk.p2_walk" "/Game/JumpOver/Sprites/Players/Player2/p2_idle.p2_idle")))
    (:NewEnumerator1
      (Sprite|SetFlipbook (Variables|Default|GetSprite) "/Game/JumpOver/Sprites/Players/Player2/p2_jump.p2_jump"))
    (:NewEnumerator4
      (Sprite|SetFlipbook (Variables|Default|GetSprite) "/Game/JumpOver/Sprites/Players/Player2/p2_hit.p2_hit"))))

(event Custom|Points%20System
  (params (Valor :type Integer))
  ;[1 1 1] Points System
  (Variables|Default|Setpontos (+ Valor (Variables|Default|Getpontos))))

(event EventTick
  (params (DeltaSeconds :type Float%20%28single-precision%29))
  ;[1 1 1] Tick - Updates animation
  (Utilities|FlowControl|Sequence
    (:then_0
      (CallFunction|UpdateAnimation)
      (Math|Float|CompareFloat (.X (Math|Vector|BreakVector (Variables|/Script/Engine.MovementComponent|GetVelocity (Pawn|GetMovementComponent)))) 0.0
        (:>
          (Pawn|SetControlRotation (Pawn|GetController) (Math|Rotator|MakeRotator 0.0 0.0 0.0))
          (Variables|Default|Setfacing 1))
        (:<
          (Pawn|SetControlRotation (Pawn|GetController) (Math|Rotator|MakeRotator 0.0 0.0 1.8e+02))
          (Variables|Default|Setfacing -1))))
    (:then_1
      (CallFunction|DanoEvent))))

(event EventOnLanded
  (params (Hit :type Hit%20Result%20Structure%20%28by%20ref%29))
  ;[1 1 1] Evento ao Aterrissar
  (if (Variables|Default|GetisHit)
    (Variables|Default|Setstates "NewEnumerator5")
    (CallFunction|UpdateAnimation)
    (Utilities|FlowControl|Delay 0.5)
    (Variables|Default|Setstates "NewEnumerator0")
    (CallFunction|UpdateAnimation)
    (Input|EnableInput (Game|GetPlayerController 0))
    (Variables|Default|SetisHit false)
    (else
      (Variables|Default|Setstates "NewEnumerator0")
      (CallFunction|UpdateAnimation))))

(event EventBeginPlay
  (Utilities|FlowControl|Sequence
    (:then_0
      (Class|ActorComponent|SetIsReplicated (Variables|Default|GetSprite) true))))

(fn ConstructionScript)