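; EnemyAIManual is a 2D sprite enemy character that chases visible pawns, attacking with a jump.
; Each Tick updates the flipbook from its state, faces the movement direction and scans for targets.
; A sphere trace gathers nearby pawns, excluding other EnemyAIManual actors, and a line trace confirms sight.
; MoveTo uses SimpleMoveToLocation, jumping when close or, after a delay, when heights differ; the airborne damage trace's result is unused.
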(event Custom|Move%20To
  (params (Goal :type Actor%20Object%20Reference))
  (bind _returnvalue (Transformation|GetActorLocation Goal))
  (bind _self self)
  (bind _returnvalue_2 (Pawn|GetController _self))
  (if (<= (Math|Float|Round (Class|Actor|GetVerticalDistanceto Goal)) 3)
    (AI|Navigation|SimpleMovetoLocation _returnvalue_2 _returnvalue)
    (if (< (Transformation|GetHorizontalDistanceTo Goal) 1e+02)
      (CallFunction|Atacar))
    (else
      (AI|Navigation|SimpleMovetoLocation _returnvalue_2 _returnvalue)
      (Utilities|FlowControl|Delay 0.5)
      (Character|Jump))))

(event Custom|Sprint
  (params (value :type Float%20%28single-precision%29))
  ;[1 1 1] Handle movement
)

(event Custom|Atacar
  (Character|Jump))

(event Custom|UpdateAnimation
  ;[1 1 1] Handle Animation
  (switch Utilities|FlowControl|Switch|Switchonstates_player (Variables|Default|Getstates)
    (:NewEnumerator0
      (Sprite|SetFlipbook (Variables|Default|GetSprite) (select (> (Math|Vector|VectorLength (Transformation|GetVelocity)) 0.0) "/Game/JumpOver/Sprites/Players/Player1/Walk/p1_walk_0.p1_walk_0" "/Game/JumpOver/Sprites/Players/Player1/p1_idle.p1_idle")))
    (:NewEnumerator1
      (Sprite|SetFlipbook (Variables|Default|GetSprite) "/Game/JumpOver/Sprites/Players/Player1/p1_jump.p1_jump"))
    (:NewEnumerator4
      (Sprite|SetFlipbook (Variables|Default|GetSprite) "/Game/JumpOver/Sprites/Players/Player1/p1_hit.p1_hit"))
    (:NewEnumerator7
      (Sprite|SetFlipbook (Variables|Default|GetSprite) "/Game/JumpOver/Sprites/Players/Player1/p1_kneel.p1_kneel"))))

(event Custom|Event%20Dano
  (bind _self self)
  (bind _returnvalue (Transformation|GetActorLocation _self))
  ;[1 1 1] Event Dano
  (if (not (AI|Components|NavMovement|IsMovingonGround (Variables|Character|GetCharacterMovement)))
    (bind _outhit (Collision|LineTraceForObjects _returnvalue (+ _returnvalue (* (Transformation|GetActorUpVector _self) (Variables|Default|GetTraceLength))) (Utilities|Array|MakeArray "ObjectTypeQuery1" "ObjectTypeQuery3") false 0 "None"))))

(event Custom|MoveRight
  (params (NewParam :type Float%20%28single-precision%29))
  (bind _velocidade (Variables|Default|Getvelocidade))
  ;[1 1 1] Handle movement
  (Pawn|Input|AddMovementInput "1.000000, 0, 0" (* (/ NewParam (Variables|Default|Getvelocidade)) (Math|Float|Clamp(Float) (* (stale Custom|Sprint value) _velocidade) (Variables|Default|GetvelocidadeCaminhando) _velocidade)) false))

(event Custom|Points%20System
  (params (Valor :type Integer))
  ;[1 1 1] Points System
  (Variables|Default|Setpontos (+ Valor (Variables|Default|Getpontos))))

(event Custom|Check%20Enemies
  (bind _self self)
  (bind _returnvalue (Transformation|GetActorLocation _self))
  (bind _outactors (Actor|GetAllActorsOfClass "EnemyAIManual_C"))
  (bind _outhits (Collision|MultiSphereTraceForObjects _returnvalue (+ _returnvalue "0, 0,15.000000") 1.5e+03 (Utilities|Array|MakeArray "ObjectTypeQuery3") false _outactors "None"))
  (bind _array_element (Utilities|Array|ForEachLoopwithBreak _outhits)
    (:LoopBody
      (bind _outhit (Collision|LineTraceByChannel (Transformation|GetActorLocation self) (Transformation|GetActorLocation (.HitActor (Collision|BreakHitResult _array_element))) "TraceTypeQuery2" false _outactors "None"))
      (if (== (.HitActor (Collision|BreakHitResult _outhit)) (.HitActor (Collision|BreakHitResult _array_element)))
        (CallFunction|Moveto (.HitActor (Collision|BreakHitResult _outhit)))))))

(event EventTick
  (params (DeltaSeconds :type Float%20%28single-precision%29))
  ;[1 1 1] Tick - Updates animation
  (Utilities|FlowControl|Sequence
    (:then_0
      (CallFunction|EventDano))
    (:then_1
      (CallFunction|UpdateAnimation)
      (Math|Float|CompareFloat (.X (Math|Vector|BreakVector (Variables|/Script/Engine.MovementComponent|GetVelocity (Pawn|GetMovementComponent)))) 0.0
        (:>
          (Pawn|SetControlRotation (Pawn|GetController) (Math|Rotator|MakeRotator 0.0 0.0 0.0))
          (Variables|Default|Setfacing 1))
        (:<
          (Pawn|SetControlRotation (Pawn|GetController) (Math|Rotator|MakeRotator 0.0 0.0 1.8e+02))
          (Variables|Default|Setfacing -1))))
    (:then_2
      (CallFunction|CheckEnemies))))

(event EventOnLanded
  (params (Hit :type Hit%20Result%20Structure%20%28by%20ref%29))
  ;[1 1 1] Evento ao Aterrissar
  (if (Variables|Default|GetisHit)
    (Variables|Default|Setstates "NewEnumerator5")
    (CallFunction|UpdateAnimation)
    (Utilities|FlowControl|Delay 0.5)
    (Variables|Default|Setstates "NewEnumerator0")
    (CallFunction|UpdateAnimation)
    (Input|EnableInput (Game|GetPlayerController 0))
    (Variables|Default|SetisHit false)
    (else
      (Variables|Default|Setstates "NewEnumerator0")
      (CallFunction|UpdateAnimation))))

(event EventBeginPlay
  (Class|ActorComponent|SetIsReplicated (Variables|Default|GetSprite) true))

(fn ConstructionScript)

(fn DebugWalkBot
  (params (InInt :type Integer) (InInt2 :type Integer))
  (Development|PrintString (Utilities|String|Append "Goal: " (Utilities|String|ToString(Integer) InInt) "  Origin: " (Utilities|String|ToString(Integer) InInt2)) true false)
  (return))