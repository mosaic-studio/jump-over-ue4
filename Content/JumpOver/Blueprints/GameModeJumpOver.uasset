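; Game mode for JumpOver that resets the player character when it is killed.
; On BeginPlay or Respawn it casts player character 0 to Player and binds to its KillPlayer dispatcher.
; When that fires, the same pawn moves back to its LocalOrigem position, becomes visible and regains collision.
; A delayed spawn-and-possess respawn chain is left unconnected, so no new pawn is spawned.
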(event Custom|Kill%20Player_Event_0
  (Transformation|SetActorLocation (stale Custom|Respawn _asplayer) (Variables|/Game/JumpOver/Blueprints/Player.Player_C|GetlocalOrigem (stale Custom|Respawn _asplayer)) false false)
  (Rendering|SetActorHiddenInGame (stale Custom|Respawn _asplayer) false)
  (Collision|SetActorEnableCollision (stale Custom|Respawn _asplayer) true))

(event Custom|Respawn
  (bind _asplayer (Utilities|Casting|CastToPlayer (Game|GetPlayerCharacter 0)))
  (EventDispatchers|AssignKillPlayer _asplayer (delegate Custom|Kill%20Player_Event_0)))

(event EventBeginPlay
  (bind _asplayer (Utilities|Casting|CastToPlayer (Game|GetPlayerCharacter 0)))
  (EventDispatchers|AssignKillPlayer _asplayer (delegate Custom|Kill%20Player_Event_0)))

(event EventTick
  (params (DeltaSeconds :type Float%20%28single-precision%29)))

(fn ConstructionScript)