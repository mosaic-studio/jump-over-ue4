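; Enemy2 is a Paper2D enemy character for the JumpOver game, handling sprite animation and facing, with its capsule component set to replicate on begin play.
; Each tick it selects a P2 flipbook from its state (Idle, Jumping or Hit), with Idle switching between walk and idle by velocity.
; It then turns the controller yaw and updates Facing from the sign of horizontal X velocity.
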(event Custom|UpdateAnimation
  (switch Utilities|FlowControl|Switch|Switchonstates_player (Variables|Default|Getstates)
    (:NewEnumerator0
      (Sprite|SetFlipbook (Variables|Default|GetPaperFlipbook) (select (> (Math|Vector|VectorLength (Transformation|GetVelocity)) 0.0) "/Game/JumpOver/Sprites/Players/Player2/p2_walk.p2_walk" "/Game/JumpOver/Sprites/Players/Player2/p2_idle.p2_idle")))
    (:NewEnumerator1
      (Sprite|SetFlipbook (Variables|Default|GetPaperFlipbook) "/Game/JumpOver/Sprites/Players/Player2/p2_jump.p2_jump"))
    (:NewEnumerator4
      (Sprite|SetFlipbook (Variables|Default|GetPaperFlipbook) "/Game/JumpOver/Sprites/Players/Player2/p2_hit.p2_hit"))))

(event EventBeginPlay
  (Class|ActorComponent|SetIsReplicated (Variables|Default|GetCapsule) true))

(event EventActorBeginOverlap
  (params (OtherActor :type Actor%20Object%20Reference)))

(event EventTick
  (params (DeltaSeconds :type Float%20%28single-precision%29))
  (Utilities|FlowControl|Sequence
    (:then_0
      (CallFunction|UpdateAnimation)
      (Math|Float|CompareFloat (.X (Math|Vector|BreakVector (Variables|/Script/Engine.MovementComponent|GetVelocity (Pawn|GetMovementComponent)))) 0.0
        (:>
          (Pawn|SetControlRotation (Pawn|GetController) (Math|Rotator|MakeRotator 0.0 0.0 0.0))
          (Variables|Default|Setfacing 1))
        (:<
          (Pawn|SetControlRotation (Pawn|GetController) (Math|Rotator|MakeRotator 0.0 0.0 1.8e+02))
          (Variables|Default|Setfacing -1))))))

(fn ConstructionScript)